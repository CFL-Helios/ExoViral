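; Explosive projectile, apparently a launcher grenade, that deals radial damage on hit.
; Shortly after BeginPlay, it sets its ProjectileMovement velocity from HitVelocity.
; On hit, it stops the Niagara trail, plays explosion sound and effects, removes its sphere and applies falloff damage at the hit location.
; It draws debug spheres for both damage radii, then destroys itself after a short delay.
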(event `self.ReceiveBeginPlay`
  (`KismetSystemLibrary.Delay` 0.2)
  (set `MovementComponent.Velocity` (`self.HitVelocity`) (`self.ProjectileMovement`)))

(event `self.ReceiveHit`
  (params (MyComp :type "PrimitiveComponent Object Reference") (Other :type "Actor Object Reference") (OtherComp :type "PrimitiveComponent Object Reference") (bSelfMoved :type Boolean) (HitLocation :type "Vector Structure") (HitNormal :type "Vector Structure") (NormalImpulse :type "Vector Structure") (Hit :type "HitResult Structure (by ref)"))
  (bind _hitlocation (`self.HitLocation`))
  ;[1 1 1] Deactivate Smoke Trail On Hit
  (`ActorComponent.Deactivate` (`self.Niagara`))
  (set `self.HitLocation` HitLocation)
  (`GameplayStatics.PlaySoundAtLocation` "/Game/MilitaryWeapDark/Sound/GrenadeLauncher/GrenadeLauncher_Explosion_Cue.GrenadeLauncher_Explosion_Cue" (`self.HitLocation`) (struct) 1.0 1.0 0.0 "/Game/MilitaryWeapDark/Sound/Attenuation/Explosion_att.Explosion_att" null null null)
  ;[1 1 1] Spawn Explosion Effects
  (`NiagaraFunctionLibrary.SpawnSystemAtLocation` "/Game/Projectiles/P_GrenadeExplosion.P_GrenadeExplosion" (`self.HitLocation`))
  (`ActorComponent.K2_DestroyComponent` (`self.Sphere1`))
  ;[1 1 1] Apply Damage
  (`GameplayStatics.ApplyRadialDamageWithFalloff` :`BaseDamage` 50.0 :`MinimumDamage` 25.0 :`Origin` (`self.HitLocation`) :`DamageInnerRadius` 200.0 :`DamageOuterRadius` 350.0 :`DamageFalloff` 1.0 :`DamageCauser` null :`InstigatedByController` null)
  (`KismetSystemLibrary.DrawDebugSphere` _hitlocation 200.0 12 (struct :`R` 1.0 :`G` 1.0 :`B` 1.0 :`A` 1.0) 2.0 1.0)
  (`KismetSystemLibrary.DrawDebugSphere` _hitlocation 350.0 12 (struct :`R` 1.0 :`G` 1.0 :`B` 1.0 :`A` 1.0) 2.0 1.0)
  (`KismetSystemLibrary.Delay` 1.0)
  (`self.K2_DestroyActor`))

(fn `UserConstructionScript`)