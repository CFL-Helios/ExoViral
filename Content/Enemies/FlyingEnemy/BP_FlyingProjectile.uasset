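; Homing projectile for the flying enemy that chases the player character and deals damage on impact.
; On BeginPlay it sets a scene component of the player as the projectile movement's homing target, with acceleration from HomingSpeed, then starts a self-destruct timer.
; A hit damages either the player or a BP_Enemy, and any hit destroys the projectile.
; Any damage taken also destroys it, so it can be shot down.
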(event `self.ReceiveBeginPlay`
  (`self.Lock On`)
  (`self.Destruction Countdown`))

(event `Lock On`
  (bind _projectilemovement (`self.ProjectileMovement`))
  ;[1 1 1] Lock on to target
  (bind _homing_target (`self.Find Homing Target`))
  (set `ProjectileMovementComponent.HomingTargetComponent` _homing_target _projectilemovement)
  (set `ProjectileMovementComponent.bIsHomingProjectile` true _projectilemovement)
  (set `ProjectileMovementComponent.HomingAccelerationMagnitude` (`self.Homing Speed`) (`self.ProjectileMovement`)))

(event `self.ReceiveAnyDamage`
  (params (Damage :type "Float (single-precision)") (DamageType :type "DamageType Object Reference") (InstigatedBy :type "Controller Object Reference") (DamageCauser :type "Actor Object Reference"))
  (`self.K2_DestroyActor`))

(event `Destruction Countdown`
  ;[1 1 1] Destroys projectile, if hasn't hit player in X amount of time
  (`KismetSystemLibrary.Delay` (`self.TimeToSelfDestruct`))
  (`self.K2_DestroyActor`))

(event `self.ReceiveHit`
  (params (MyComp :type "PrimitiveComponent Object Reference") (Other :type "Actor Object Reference") (OtherComp :type "PrimitiveComponent Object Reference") (bSelfMoved :type Boolean) (HitLocation :type "Vector Structure") (HitNormal :type "Vector Structure") (NormalImpulse :type "Vector Structure") (Hit :type "HitResult Structure (by ref)"))
  (bind _attackdamage (`self.AttackDamage`))
  ;[1 1 1] Apply damage to player on hit, then destroy actor
  (bind _asbp_third_person_character (cast `/Game/Player/BP_ThirdPersonCharacter` Other)
    (:`then`
      (`GameplayStatics.ApplyDamage` _asbp_third_person_character _attackdamage null self))
    (:`CastFailed`
      (bind _asbp_enemy (cast `/Game/Enemies/GroundEnemy/BP_Enemy` Other)
        (:`then`
          (`GameplayStatics.ApplyDamage` _asbp_enemy _attackdamage null self))
        (:`CastFailed`
          _))))
  (`self.K2_DestroyActor`))

(fn `Find Homing Target`
  (returns (`Homing Target` :type "SceneComponent Object Reference") (`Target Location` :type "Vector Structure"))
  (bind _asbp_third_person_character (cast `/Game/Player/BP_ThirdPersonCharacter` (`GameplayStatics.GetPlayerCharacter` 0)))
  (bind _output_get (set `self.Homing Target` _asbp_third_person_character))
  (bind _output_get_2 (set `self.target location` (`self.K2_GetActorLocation` _asbp_third_person_character)))
  (return (`self.GetComponentByClass` _output_get "/Script/Engine.SceneComponent") _output_get_2))

(fn `UserConstructionScript`)