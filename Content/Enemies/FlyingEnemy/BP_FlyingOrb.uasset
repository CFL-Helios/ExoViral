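; BP_FlyingOrb is a flying enemy that shoots projectiles and can be destroyed by damage.
; On BeginPlay it starts the FlyingAI_BT behavior tree, then enters a looping delay that periodically calls FireProjectile, independent of the tree.
; FireProjectile spawns BP_FlyingProjectile at the SpawnPointRef location, setting no rotation.
; AnyDamage subtracts from Health and destroys the actor once it drops below zero.
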(event `self.ReceiveBeginPlay`
  (`AIController.RunBehaviorTree` (`AIBlueprintHelperLibrary.GetAIController` self) "/Game/Enemies/FlyingEnemy/FlyingAI_BT.FlyingAI_BT")
  (`KismetSystemLibrary.Delay` 5.0 :!label _label)
  (`self.Fire Projectile`)
  (goto _label))

(event `self.ReceiveAnyDamage`
  (params (Damage :type "Float (single-precision)") (DamageType :type "DamageType Object Reference") (InstigatedBy :type "Controller Object Reference") (DamageCauser :type "Actor Object Reference"))
  ;[1 1 1] Enemy take damage
  (bind _output_get (set `self.Health` (- (`self.Health`) Damage)))
  (if (< _output_get 0.0)
    (`self.K2_DestroyActor`)))

(event `Fire Projectile`
  (`|SpawnActorFromClass` "/Game/Enemies/FlyingEnemy/BP_FlyingProjectile.BP_FlyingProjectile_C" (`KismetMathLibrary.MakeTransform` (`SceneComponent.K2_GetComponentLocation` (`self.SpawnPointRef`))) "Undefined" "MultiplyWithRoot" null null))

(fn `UserConstructionScript`)