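; BP_FlyingEnemy is a flying enemy that repeatedly fires projectiles while its AI controller runs the FlyingAI_BT behavior tree.
; On BeginPlay it calls the parent logic, teleports up by StartHeight from its capsule location and starts the behavior tree.
; A self-calling, delayed event spawns BP_FlyingProjectile at the spawn point every FireRate seconds and passes it CurrentDamage, independent of any target check in this graph.
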(event `self.ReceiveBeginPlay`
  (bind (_returnvalue_x _returnvalue_y _returnvalue_z) (`KismetMathLibrary.BreakVector` (`SceneComponent.K2_GetComponentLocation` (`self.CapsuleComponent`))))
  (`parent.ReceiveBeginPlay`)
  (`self.K2_TeleportTo` (`KismetMathLibrary.MakeVector` _returnvalue_x _returnvalue_y (+ _returnvalue_z (`self.StartHeight`))))
  (`AIController.RunBehaviorTree` (`AIBlueprintHelperLibrary.GetAIController` self) "/Game/Enemies/FlyingEnemy/FlyingAI_BT.FlyingAI_BT")
  ;[1 1 1] Establishes Projectile Spawn Loop
  (`KismetSystemLibrary.Delay` (`self.Fire Rate`))
  (`self.Fire Projectile`))

(event `Fire Projectile`
  ;[1 1 1] Spawns Homing Projectile Loop
  (bind _returnvalue (`|SpawnActorFromClass` "/Game/Enemies/FlyingEnemy/BP_FlyingProjectile.BP_FlyingProjectile_C" (`KismetMathLibrary.MakeTransform` (`SceneComponent.K2_GetComponentLocation` (`self.SpawnPointRef`))) "Undefined" "MultiplyWithRoot" null null))
  (set `/Game/Enemies/FlyingEnemy/BP_FlyingProjectile.AttackDamage` (`self.CurrentDamage`) _returnvalue)
  (`KismetSystemLibrary.Delay` (`self.Fire Rate`))
  (`self.Fire Projectile`))

(fn `UserConstructionScript`
  (`parent.UserConstructionScript`))