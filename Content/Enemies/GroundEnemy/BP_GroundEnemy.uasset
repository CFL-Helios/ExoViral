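; BP_GroundEnemy is a ground enemy with a melee attack against characters in range.
; Its Attack event applies Damage to every Character overlapping AttackBox, excluding itself.
; The attack sound and cross-slice montage play inside that loop, so they trigger once per target hit and not at all on a miss.
; BeginPlay and the construction script add no logic of their own.
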(event `Attack`
  ;[1 1 1] Attack Player
  (for _array_element (`PrimitiveComponent.GetOverlappingActors` (`self.AttackBox`) "/Script/Engine.Character")
    (if (!= _array_element self)
      (`GameplayStatics.ApplyDamage` _array_element (`self.Damage`) null self)
      (`GameplayStatics.SpawnSoundAttached` "/Game/Audio/SFX/ENEMY_SFX/Aeromorph/SC_AeromorphAttack.SC_AeromorphAttack" (`self.CapsuleComponent`) "None" (0.0 0.0 0.0) (struct) "KeepRelativeOffset" false 1.0 1.0 0.0 null null)
      (`|PlayMontage` (`self.Mesh`) "/Game/Enemies/GroundEnemy/Animation/Monster_CrossSlice_Attack_Anim_Montage.Monster_CrossSlice_Attack_Anim_Montage"))))

(fn `UserConstructionScript`
  (`parent.UserConstructionScript`))