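; BP_Enemy is a ground enemy that can damage the player and be destroyed by damage.
; Its Attack event, with no caller in this file, applies damage to every third-person character overlapping the AttackBox.
; Incoming damage is subtracted from Health, and the actor destroys itself only when Health drops below zero, so exactly zero survives.
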(event `Attack`
  ;[1 1 1] Attack Player
  (for _array_element (`PrimitiveComponent.GetOverlappingActors` (`self.AttackBox`) "/Game/Player/BP_ThirdPersonCharacter.BP_ThirdPersonCharacter_C")
    (bind _asactor (cast `Actor` _array_element))
    (`GameplayStatics.ApplyDamage` _asactor (`self.AtttackDamage`) null self)))

(event `self.ReceiveAnyDamage`
  (params (Damage :type "Float (single-precision)") (DamageType :type "DamageType Object Reference") (InstigatedBy :type "Controller Object Reference") (DamageCauser :type "Actor Object Reference"))
  ;[1 1 1] Take Damage
  (bind _output_get (set `self.Health` (- (`self.Health`) Damage)))
  (if (< _output_get 0.0)
    (`self.K2_DestroyActor`)))

(fn `UserConstructionScript`)