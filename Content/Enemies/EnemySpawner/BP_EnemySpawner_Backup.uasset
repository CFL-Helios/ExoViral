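; Enemy spawner that places weighted-random enemies at reachable points in its spawn area while the player is inside its trigger sphere.
; Tick drives spawning through a DoOnce re-armed after randomized delays, gated by GameMode approval and a wave count.
; GameMode level-ups reset the count and compute scaled limit and interval, though spawning reads the unscaled values.
; A debug sphere shows whether the trigger is active.
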(event `self.ReceiveBeginPlay`
  (bind _asbp_third_person_game_mode (cast `/Game/Player/BP_ThirdPersonGameMode` (`GameplayStatics.GetGameMode`)))
  (bind _output_get (set `self.GameMode` _asbp_third_person_game_mode))
  ;[1 1 1] Set Difficulty Stats
  (add `/Game/Player/BP_ThirdPersonGameMode.DifficultyLevelUp` _output_get (delegate `Set Difficulty`))
  (bind _level (`/Game/Player/BP_ThirdPersonGameMode.Get Level` _output_get))
  (`self.Set Difficulty` _level)
  ;[1 1 1] Check if Player is in Trigger Area
  (set `self.SpawnActive` (`KismetArrayLibrary.Array_IsNotEmpty` (`PrimitiveComponent.GetOverlappingActors` (`self.Trigger Range`) "/Game/Player/BP_ThirdPersonCharacter.BP_ThirdPersonCharacter_C")))
  (bind _value (`self.RandomInterval`))
  (`KismetSystemLibrary.Delay` _value)
  (`self.Ready Spawn`))

(event `Set Difficulty`
  (params (Level :type Integer))
  ;[1 1 1] Set Difficulty Stats
  (set `self.WaveCount` 0)
  (set `self.CurrentWaveLimit` (+ (* Level (`self.WavePerLevel`)) (`self.WaveLimit`)))
  (set `self.CurrentSpawnInt` (* (`KismetMathLibrary.MultiplyMultiply_FloatFloat` (`self.SpawnIntLevelMult`) (`KismetMathLibrary.Conv_IntToDouble` Level)) (`self.SpawnInterval`))))

(event `self.ReceiveTick`
  (params (DeltaSeconds :type "Float (single-precision)"))
  (bind _trigger_range (`self.Trigger Range`))
  (bind _returnvalue (`SceneComponent.K2_GetComponentLocation` _trigger_range))
  (bind _sphereradius (`SphereComponent.SphereRadius` _trigger_range))
  ;[1 1 1] Debug Sphere for Spawner
  (if (`self.SpawnActive`)
    (`KismetSystemLibrary.DrawDebugSphere` _returnvalue _sphereradius 12 (`KismetMathLibrary.LinearColor_Green`))
    (else
      (`KismetSystemLibrary.DrawDebugSphere` _returnvalue _sphereradius 12 (`KismetMathLibrary.LinearColor_White`))))
  ;[1 1 1] Attempt to Spawn Enemy
  (if (`self.SpawnActive`)
    (`self.Spawn Enemy`)))

(event `self.Trigger Range.OnComponentBeginOverlap`
  (params (OverlappedComponent :type "PrimitiveComponent Object Reference") (OtherActor :type "Actor Object Reference") (OtherComp :type "PrimitiveComponent Object Reference") (OtherBodyIndex :type Integer) (bFromSweep :type Boolean) (SweepResult :type "HitResult Structure (by ref)"))
  ;[1 1 1] Toggle Spawn Active
  (cast `/Game/Player/BP_ThirdPersonCharacter` OtherActor)
  (set `self.SpawnActive` true))

(event `self.Trigger Range.OnComponentEndOverlap`
  (params (OverlappedComponent :type "PrimitiveComponent Object Reference") (OtherActor :type "Actor Object Reference") (OtherComp :type "PrimitiveComponent Object Reference") (OtherBodyIndex :type Integer))
  ;[1 1 1] Toggle Spawn Active
  (cast `/Game/Player/BP_ThirdPersonCharacter` OtherActor)
  (set `self.SpawnActive` false))

(event `Spawn Enemy`
  (bind _spawn_area (`self.Spawn Area`))
  ;[1 1 1] Spawn Enemy
  (`/Engine/EditorBlueprintResources/StandardMacros.DoOnce` true :!label _label
    (:`Completed`
      (if (< (`self.WaveCount`) (`self.WaveLimit`))
        (bind _success (`/Game/Player/BP_ThirdPersonGameMode.Test Enemy Spawn` (`self.GameMode`)))
        (if _success
          (bind _enemy (`self.RandomEnemy`))
          (bind _returnvalue (`|SpawnActorFromClass` _enemy (`KismetMathLibrary.MakeTransform` (`NavigationSystemV1.K2_GetRandomReachablePointInRadius` (`SceneComponent.K2_GetComponentLocation` _spawn_area) (`SphereComponent.SphereRadius` _spawn_area) null null) (`KismetMathLibrary.MakeRotator` (`KismetMathLibrary.RandomFloatInRange` 0.0 360.0))) "AdjustIfPossibleButDontSpawnIfColliding" "MultiplyWithRoot" null null))
          (`/Engine/EditorBlueprintResources/StandardMacros.IsValid` _returnvalue
            (:`Is Valid`
              (`/Game/Player/BP_ThirdPersonGameMode.Add Enemy` (`self.GameMode`))
              (set `self.WaveCount` (+ (`self.WaveCount`) 1)))
            (:`Is Not Valid`
              _))))
      (bind _value (`self.RandomInterval`))
      (`KismetSystemLibrary.Delay` _value)
      (`self.Ready Spawn`))))

(event `Ready Spawn`
  ;[1 1 1] Spawn Enemy
  (goto _label :!via `Reset`))

(fn `RandomEnemy`
  (returns (Enemy :type "Character Class Reference"))
  (locals (RandomFloat :type "Float (double-precision)" :default 0.0) (CurrentChance :type "Float (double-precision)"))
  (set `local.RandomFloat` (`KismetMathLibrary.RandomFloat`))
  (for (_array_element _array_index) (`self.SpawnChances`)
    (bind _output_get (set `local.CurrentChance` (+ _array_element (`local.CurrentChance`))))
    (if (> _output_get (`local.RandomFloat`))
      (return (`|GetArrayItem` (`self.SpawnEnemies`) _array_index)))))

(fn `RandomInterval`
  (returns (Value :type "Float (double-precision)"))
  (bind _returnvalue (/ (`self.SpawnIntVariance`) 2.0))
  (return (+ (`KismetMathLibrary.RandomFloatInRange` (* -1.0 _returnvalue) _returnvalue) (`self.SpawnInterval`))))

(fn `UserConstructionScript`)