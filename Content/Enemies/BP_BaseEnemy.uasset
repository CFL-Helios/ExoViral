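; BP_BaseEnemy is the base enemy, with health and damage scaled exponentially by the game mode's difficulty level.
; Health is set from the level at spawn, while damage also updates on each DifficultyLevelUp event.
; When damage drops health below zero, it may spawn a health drop homing to a player killer, notifies the game mode, unpossesses, ragdolls and is destroyed after a short delay.
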(event `self.ReceiveBeginPlay`
  (bind _asbp_third_person_game_mode (cast `/Game/Player/BP_ThirdPersonGameMode` (`GameplayStatics.GetGameMode`)))
  (bind _output_get (set `self.GameMode` _asbp_third_person_game_mode))
  ;[1 1 1] Set Stats Based on Spawned Difficulty
  (bind _level (`/Game/Player/BP_ThirdPersonGameMode.Get Level` _output_get))
  (set `self.CurrentHealth` (* (`KismetMathLibrary.MultiplyMultiply_FloatFloat` (`self.HealthLevelMult`) (`KismetMathLibrary.Conv_IntToDouble` _level)) (`self.Health`)))
  (`self.Set Damage Level` _level)
  (add `/Game/Player/BP_ThirdPersonGameMode.DifficultyLevelUp` (`self.GameMode`) (delegate `Set Damage Level`)))

(event `Set Damage Level`
  (params (Level :type Integer))
  ;[1 1 1] Set Damaged Based on Level
  (set `self.CurrentDamage` (* (`self.Damage`) (`KismetMathLibrary.MultiplyMultiply_FloatFloat` (`self.DamageLevelMult`) (`KismetMathLibrary.Conv_IntToDouble` Level)))))

(event `self.ReceiveAnyDamage`
  (params (Damage :type "Float (single-precision)") (DamageType :type "DamageType Object Reference") (InstigatedBy :type "Controller Object Reference") (DamageCauser :type "Actor Object Reference"))
  ;[1 1 1] Take Damage
  (bind _output_get (set `self.CurrentHealth` (- (`self.CurrentHealth`) Damage)))
  (if (< _output_get 0.0)
    (`self.Die` DamageCauser)
    (else
      (`GameplayStatics.SpawnSoundAttached` (`self.DamageSound`) (`self.CapsuleComponent`) "None" (0.0 0.0 0.0) (struct) "KeepRelativeOffset" false 1.0 1.0 0.0 null null))))

(event `Die`
  (params (Killer :type "Actor Object Reference"))
  ;[1 1 1] Death
  (`self.DropTo` Killer)
  (`/Game/Player/BP_ThirdPersonGameMode.Remove Enemy` (`self.GameMode`))
  (`Controller.UnPossess` (`self.GetController`))
  (set `self.bCanBeDamaged` false)
  (`GameplayStatics.SpawnSoundAttached` (`self.DeathSound`) (`self.CapsuleComponent`) "None" (0.0 0.0 0.0) (struct) "KeepRelativeOffset" false 1.0 1.0 0.0 null null)
  (`self.Ragdoll`)
  (`KismetSystemLibrary.Delay` 2.0)
  (`self.K2_DestroyActor`))

(event `Ragdoll`
  (bind _mesh (`self.Mesh`))
  ;[1 1 1] Ragdoll
  (`PrimitiveComponent.SetSimulatePhysics` _mesh true)
  (`SkeletalMeshComponent.SetPhysicsBlendWeight` _mesh 1.0)
  (`PrimitiveComponent.SetCollisionEnabled` _mesh "QueryAndPhysics")
  (`PrimitiveComponent.SetEnableGravity` (`self.CapsuleComponent`) true))

(event `DropTo`
  (params (Actor :type "Actor Object Reference"))
  ;[1 1 1] Drop Health
  (bind _asbp_third_person_character (cast `/Game/Player/BP_ThirdPersonCharacter` Actor))
  (if (< (`KismetMathLibrary.RandomFloat`) (`self.DropChance`))
    (bind _returnvalue (`|SpawnActorFromClass` "/Game/Enemies/HealthDrop/BP_HealthDrop.BP_HealthDrop_C" (`self.GetTransform`) "AlwaysSpawn" "MultiplyWithRoot" null _asbp_third_person_character))
    (set `ProjectileMovementComponent.HomingTargetComponent` (`Actor.RootComponent` _asbp_third_person_character) (`/Game/Enemies/HealthDrop/BP_HealthDrop.ProjectileMovement` _returnvalue))))

(fn `UserConstructionScript`)