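; BP_MeshSpawner scatters randomly scaled BP_IsolatedSpawner actors across navigable terrain at startup.
; Starting from its arrow, it chains random navmesh points, searching a wide radius around each previous point.
; After each spawn, an overlap check on the new actor's arrow either calls DestroyActor on the spawner itself and retries immediately, or decrements SpawnCounter and continues after a short delay until the count runs out.
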(event `self.ReceiveBeginPlay`
  (`KismetSystemLibrary.Delay` 0.2)
  (`self.Set First Point`))

(event `Set First Point`
  (bind _randomlocation (`NavigationSystemV1.K2_GetRandomLocationInNavigableRadius` (`SceneComponent.K2_GetComponentLocation` (`self.Arrow`)) 15000.0 null null))
  (set `self.SpawnPoint` _randomlocation)
  (`self.Spawn Mesh`))

(event `Spawn Mesh`
  (bind _returnvalue (`KismetMathLibrary.RandomFloatInRange` 1.0 5.0))
  (bind _returnvalue_2 (`|SpawnActorFromClass` "/Game/ProceduralLandscape/BP_IsolatedSpawner.BP_IsolatedSpawner_C" (`KismetMathLibrary.MakeTransform` (`self.SpawnPoint`) (struct) (`KismetMathLibrary.MakeVector` _returnvalue _returnvalue _returnvalue)) "Undefined" "MultiplyWithRoot" null null))
  (if (`PrimitiveComponent.IsOverlappingActor` (`/Game/ProceduralLandscape/BP_IsolatedSpawner.Arrow` _returnvalue_2) null)
    (`self.K2_DestroyActor`)
    (`self.Set New Point`)
    (else
      (bind _output_get (set `self.SpawnCounter` (- (`self.SpawnCounter`) 1)))
      (`KismetSystemLibrary.PrintString` (`KismetStringLibrary.Conv_IntToString` _output_get))
      (if (not (<= (`self.SpawnCounter`) 1))
        (`KismetSystemLibrary.Delay` 0.2)
        (`self.Set New Point`)))))

(event `Set New Point`
  (bind _randomlocation (`NavigationSystemV1.K2_GetRandomLocationInNavigableRadius` (`self.SpawnPoint`) 15000.0 null null))
  (set `self.SpawnPoint` _randomlocation)
  (`self.Spawn Mesh`))

(fn `UserConstructionScript`)