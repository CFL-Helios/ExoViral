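; BP_DamageUpgrade is a pickup upgrade that doubles the active player's weapon damage.
; Its UpgradeEffect event multiplies both PrimaryDamage and SecondaryDamage on ActivePlayer by two.
; Its SetText event sets the displayed item description, and the construction script only calls the parent's, leaving shared pickup behavior to the parent class.
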(event `self.UpgradeEffect`
  (bind _activeplayer (`self.ActivePlayer`))
  ;[1 1 1] Effect:
  (set `/Game/Player/BP_ThirdPersonCharacter.PrimaryDamage` (* (`/Game/Player/BP_ThirdPersonCharacter.PrimaryDamage` _activeplayer) 2.0) _activeplayer)
  (set `/Game/Player/BP_ThirdPersonCharacter.SecondaryDamage` (* (`/Game/Player/BP_ThirdPersonCharacter.SecondaryDamage` _activeplayer) 2.0) _activeplayer))

(event `self.SetText`
  ;[1 1 1] Set description of item to display
  (set `self.Description` "Double Weapon Damage"))

(fn `UserConstructionScript`
  (`parent.UserConstructionScript`))