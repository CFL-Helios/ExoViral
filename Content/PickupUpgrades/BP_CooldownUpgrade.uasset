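; BP_CooldownUpgrade is a pickup upgrade that shortens the player's grenade cooldown.
; Its UpgradeEffect event scales the active player's SecondaryRate by a constant factor, so repeated applications compound.
; SetText supplies the item's display description, and the default BeginPlay, overlap and Tick events are left disabled.
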(event `self.UpgradeEffect`
  (bind _activeplayer (`self.ActivePlayer`))
  ;[1 1 1] Effect:
  (set `/Game/Player/BP_ThirdPersonCharacter.SecondaryRate` (* 0.75 (`/Game/Player/BP_ThirdPersonCharacter.SecondaryRate` _activeplayer)) _activeplayer))

(event `self.SetText`
  ;[1 1 1] Set description of item to display
  (set `self.Description` "25% Faster Grenade Cooldown"))

(fn `UserConstructionScript`
  (`parent.UserConstructionScript`))