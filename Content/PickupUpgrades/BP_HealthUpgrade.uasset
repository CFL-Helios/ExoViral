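; BP_HealthUpgrade is a pickup upgrade that boosts the active player's maximum health by ten percent.
; Its UpgradeEffect event multiplies MaxHealth and then fully heals the player by setting CurrentHealth to the new maximum.
; SetText supplies the description to display for the item.
; The Blueprint defines only the effect and text, with no active overlap, tick or construction logic of its own.
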(event `self.UpgradeEffect`
  (bind _activeplayer (`self.ActivePlayer`))
  ;[1 1 1] Effect:
  (bind _output_get (set `/Game/Player/BP_ThirdPersonCharacter.MaxHealth` (* (`/Game/Player/BP_ThirdPersonCharacter.MaxHealth` _activeplayer) 1.1) _activeplayer))
  (set `/Game/Player/BP_ThirdPersonCharacter.CurrentHealth` _output_get _activeplayer))

(event `self.SetText`
  ;[1 1 1] Set description of item to display
  (set `self.Description` "+10% Max Health"))

(fn `UserConstructionScript`
  (`parent.UserConstructionScript`))