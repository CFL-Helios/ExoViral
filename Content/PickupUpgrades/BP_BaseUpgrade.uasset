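; BP_BaseUpgrade is the parent Blueprint for pickup upgrades the player can collect.
; On BeginPlay it creates a description widget on the viewport and calls SetText, which is left empty here.
; Overlap with the third-person character stores that player and shows the description; ending overlap clears it.
; PickUp calls the player's Upgrade, runs the overridable UpgradeEffect hook, then destroys the actor.
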(event `self.ReceiveBeginPlay`
  ;[1 1 1] Create widget and set description
  (bind _returnvalue (`|CreateWidget` "/Game/Widgets/WBP_Upgrade_Description.WBP_Upgrade_Description_C"))
  (bind _output_get (set `self.DescriptionPopup` _returnvalue))
  (`UserWidget.AddToViewport` _output_get 0)
  (`self.SetText`))

(event `UpgradeEffect`
  ;[1 1 1] Override effect in child classes
)

(event `SetText`
  ;[1 1 1] Override effect in child classes
)

(event `self.ReceiveActorBeginOverlap`
  (params (OtherActor :type "Actor Object Reference"))
  ;[1 1 1] OnOverlap: Pop-up UI for description and pick-up prompt
  (bind _asbp_third_person_character (cast `/Game/Player/BP_ThirdPersonCharacter` OtherActor))
  (set `self.ActivePlayer` _asbp_third_person_character)
  (`/Game/Widgets/WBP_Upgrade_Description.ShowDescription` (`self.DescriptionPopup`) (`self.Description`)))

(event `self.ReceiveActorEndOverlap`
  (params (OtherActor :type "Actor Object Reference"))
  ;[1 1 1] EndOverlap: Remove Pop-up
  (cast `/Game/Player/BP_ThirdPersonCharacter` OtherActor)
  (`/Game/Widgets/WBP_Upgrade_Description.ShowDescription` (`self.DescriptionPopup`) ""))

(event `/Game/PickupUpgrades/BPI_PickUp.PickUp`
  ;[1 1 1] Pick-up upgrade: upgrade in effect and destroy actor
  (`/Game/Player/BP_ThirdPersonCharacter.Upgrade` (`self.ActivePlayer`))
  (`self.UpgradeEffect`)
  (`self.K2_DestroyActor`)
  (`KismetSystemLibrary.PrintString` "picked"))

(fn `UserConstructionScript`)