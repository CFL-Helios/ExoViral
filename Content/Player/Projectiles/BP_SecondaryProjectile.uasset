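; Secondary-fire explosive projectile for the player that detonates on hit.
; On hit it disables collision, stops its Niagara smoke trail, and spawns explosion sound and particles at the impact point.
; It applies radial damage with falloff down to half base damage, draws debug spheres for both radii, then destroys itself after a short delay.
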(event `self.ReceiveHit`
  (params (MyComp :type "PrimitiveComponent Object Reference") (Other :type "Actor Object Reference") (OtherComp :type "PrimitiveComponent Object Reference") (bSelfMoved :type Boolean) (HitLocation :type "Vector Structure") (HitNormal :type "Vector Structure") (NormalImpulse :type "Vector Structure") (Hit :type "HitResult Structure (by ref)"))
  (bind _base_damage (`self.Base Damage`))
  (`PrimitiveComponent.SetCollisionEnabled` (`self.Collision`) "NoCollision")
  ;[1 1 1] Deactivate Smoke Trail On Hit
  (`ActorComponent.Deactivate` (`self.Niagara`))
  ;[1 1 1] Spawn Explosion Effects
  (`GameplayStatics.PlaySoundAtLocation` "/Game/Audio/SFX/Secondary_Weapon/Helios_SFX_Secondary_Explosion.Helios_SFX_Secondary_Explosion" HitLocation (struct) 1.0 1.0 0.0 "/Game/MilitaryWeapDark/Sound/Attenuation/Explosion_att.Explosion_att" null null null)
  (`NiagaraFunctionLibrary.SpawnSystemAtLocation` "/Game/Player/Projectiles/P_GrenadeExplosion.P_GrenadeExplosion" HitLocation)
  (`GameplayStatics.ApplyRadialDamageWithFalloff` :`BaseDamage` _base_damage :`MinimumDamage` (/ _base_damage 2.0) :`Origin` HitLocation :`DamageInnerRadius` 200.0 :`DamageOuterRadius` 350.0 :`DamageFalloff` 1.0 :`DamageCauser` self :`InstigatedByController` null)
  (`KismetSystemLibrary.DrawDebugSphere` HitLocation 200.0 12 (struct :`R` 1.0 :`G` 1.0 :`B` 1.0 :`A` 1.0) 2.0 1.0)
  (`KismetSystemLibrary.DrawDebugSphere` HitLocation 350.0 12 (struct :`R` 1.0 :`G` 1.0 :`B` 1.0 :`A` 1.0) 2.0 1.0)
  (`KismetSystemLibrary.Delay` 1.0)
  (`self.K2_DestroyActor`))

(fn `UserConstructionScript`)