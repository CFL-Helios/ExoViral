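; BP_Enemy is an AI-controlled enemy that detects the player and deals damage at close range.
; PawnSensing sets the SeesPlayer blackboard key when it sees a BP_ThirdPersonCharacter, and nothing here clears it.
; The Attack event, which has no caller in this file, applies damage to player 0 only if that character overlaps the AttackRange component.
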(event `Attack`
  (bind _returnvalue (`GameplayStatics.GetPlayerCharacter` 0))
  (if (`KismetArrayLibrary.Array_Contains` (`PrimitiveComponent.GetOverlappingActors` (`self.AttackRange`) null) _returnvalue)
    (`GameplayStatics.ApplyDamage` _returnvalue (`self.AtttackDamage`) null self)))

(event `self.PawnSensing.OnSeePawn`
  (params (Pawn :type "Pawn Object Reference"))
  (cast `/Game/Blueprints/BP_ThirdPersonCharacter` Pawn)
  (`BlackboardComponent.SetValueAsBool` (`AIBlueprintHelperLibrary.GetBlackboard` null) "SeesPlayer" true))

(fn `UserConstructionScript`)